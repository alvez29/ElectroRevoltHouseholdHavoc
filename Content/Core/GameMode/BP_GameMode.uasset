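; Game mode for a round-based wave game that spawns kitchen and household appliance enemies and manages the HUD and game-over screen.
; Timers drive pre-round and spawning phases from per-round data table rows, randomly placing toasters, microwaves or razors within a box.
; After spawning stops, a looping check advances the round once no enemies remain.
; Kills raise the music BPM parameter, and game over reverses a timeline tied to lowpass cutoff.
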(event Custom|StartPreRound
  (Utilities|LoadRoundStat
    (:Row%20Found
      (Utilities|Time|SetTimerbyEvent (delegate Custom|OnPreRoundTimeEnded) (.preroundtime (Variables|Default|GetCurrentRoundStats)))
      (Development|PrintString "Pre-round"))
    (:RowNotFound
      (Development|PrintString "You reached the end!"))))

(event Custom|OnEndCurrentRound
  ;[1 1 1] Stops spawning enemies
  (Utilities|Time|ClearandInvalidateTimerbyHandle (Variables|Default|GetSpawnEnemyTimer))
  (bind _returnvalue (Utilities|Time|SetTimerbyEvent (delegate Custom|CheckIfEnded) 2.0 true))
  (Variables|Default|SetCheckIfEndedTimer _returnvalue))

(event Custom|OnPreRoundTimeEnded
  (CallFunction|StartCurrentRound))

(event Custom|StartCurrentRound
  (bind _currentroundstats (Variables|Default|GetCurrentRoundStats))
  (Development|PrintString "Current round")
  ;[1 1 1] Rount timer
  (Utilities|Time|SetTimerbyEvent (delegate Custom|OnEndCurrentRound) (.roundtime _currentroundstats))
  ;[1 1 1] Spawn enemy
  (bind _returnvalue (Utilities|Time|SetTimerbyEvent (delegate Custom|SpawnEnemy) (.enemyspawntime _currentroundstats) true))
  (Variables|Default|SetSpawnEnemyTimer _returnvalue))

(event Custom|SpawnEnemy
  (Utilities|TrySpawnEnemy
    (:OnToaster
      _)
    (:OnMicrowave
      _)
    (:OnRazor%20%20
      _))
  (Utilities|UpdateHUDEnemiesLeft))

(event Custom|CheckIfEnded
  (bind _currentenemiesinround (Variables|Default|GetCurrentEnemiesInRound))
  (Development|PrintString (Utilities|String|ToString(Integer) _currentenemiesinround))
  (if (== _currentenemiesinround 0)
    (Default|CallOnRoundWon)
    ;[1 1 1] Increment round and start timer for pre round
    (Math|Integer|IncrementInt (Variables|Default|GetRound)
      (:%20%20
        (Utilities|UpdateHUDRound)
        (Audio|PlaySound2D "/Game/Sound/FX/yay.yay" 1.0 1.0 0.0 0 0)
        (CallFunction|StartPreRound)
        (Utilities|Time|ClearandInvalidateTimerbyHandle (Variables|Default|GetCheckIfEndedTimer))))))

(event EventOnGameOver
  (Components|Timeline|ReversefromEnd (Variables|Default|GetCutoff))
  (bind _returnvalue (UserInterface|CreateWidget "/Game/UI/WB_GameOver.WB_GameOver_C" (Game|GetPlayerController 0)))
  (UserInterface|Viewport|AddtoViewport _returnvalue 0))

(event EventUpdateProgressBar
  (params (Percentage :type Float%20%28double-precision%29))
  (Default|UpdateSpecialAttackProgressBar (Variables|Default|GetHUD) Percentage))

(event EventBeginPlay
  (bind _returnvalue (UserInterface|CreateWidget "/Game/UI/WB_HUD.WB_HUD_C" (Game|GetPlayerController 0)))
  (bind _output_get (Variables|Default|SetHUD _returnvalue))
  (UserInterface|Viewport|AddtoViewport _output_get 0)
  (CallFunction|StartPreRound))

(event EventOnEnemyKilled
  (Math|Integer|DecrementInt (Variables|Default|GetCurrentEnemiesInRound)
    (:%20%20
      (Utilities|UpdateHUDEnemiesLeft)
      (bind _result (Math|Integer|IncrementInt (Variables|Default|GetBPM))
        (:%20%20
          (Audio|Parameter|SetFloatParameter (Variables|Default|GetAudio) "InputBPM" (Math|Conversions|ToFloat(Integer) _result) :!class /Script/AudioExtensions.AudioParameterControllerInterface))))))

(fn ConstructionScript)