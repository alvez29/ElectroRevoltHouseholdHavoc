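; Base enemy character that reports its spawn and death to the game mode and takes its movement speed from per-round stats.
; OnHurt subtracts damage from health and plays a sound, calling Die when health runs out; hurt feedback is only a placeholder print.
; Die uses a DoOnce to notify the game mode and destroy the actor a single time.
; InitRoundValues passes round stats to InitValues, which sets max walk speed.
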(event Custom|Die
  (Utilities|FlowControl|DoOnce false
    (:Completed
      (Class|BPIGameMode|OnEnemyKilled(Message) (Game|GetGameMode))
      (Actor|DestroyActor))))

(event EventBeginPlay
  (Class|BPIGameMode|OnEnemySpawn(Message) (Game|GetGameMode)))

(event EventOnHurt
  (params (Damage :type Float%20%28double-precision%29))
  (Development|PrintString "add hurt feedback")
  (bind _output_get (Variables|Default|SetHealth (- (Variables|Default|GetHealth) Damage)))
  (if (<= _output_get 0.0)
    (CallFunction|Die)
    (Audio|PlaySound2D "/Game/Sound/FX/fart.fart" 1.0 1.0 0.0 0 0)
    (else
      (Audio|PlaySound2D "/Game/Sound/FX/target.target" 1.0 1.0 0.0 0 0))))

(event EventInitRoundValues
  (params (RoundStats :type S%20Round%20Stat%20Structure))
  (CallFunction|InitValues RoundStats))

(fn ConstructionScript)

(fn InitValues
  (params (RoundStats :type S%20Round%20Stat%20Structure))
  (Utilities|FlowControl|Sequence
    (:then_0
      (Variables|/Script/Engine.CharacterMovementComponent|SetMaxWalkSpeed (Variables|Character|GetCharacterMovement) (.enemyspeed RoundStats)))))