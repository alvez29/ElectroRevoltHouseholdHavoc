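; BP_Razor is an enemy hazard that glides across the XY plane, bouncing off walls and killing the player on contact.
; It starts in a random direction and moves every Tick at a speed set from round stats.
; Separate X and Y colliders flip that direction axis on "Wall"-tagged overlaps and re-aim the actor.
; A damage collider sends KillMessage through BPI_PlayerInteraction; a mesh-floating Timeline exists but never runs.
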(event OnComponentBeginOverlap(YCollision)
  (params (OverlappedComponent :type Primitive%20Component%20Object%20Reference) (OtherActor :type Actor%20Object%20Reference) (OtherComp :type Primitive%20Component%20Object%20Reference) (OtherBodyIndex :type Integer) (bFromSweep :type Boolean) (SweepResult :type Hit%20Result%20Structure%20%28by%20ref%29))
  (bind _returnvalue (Transformation|GetActorLocation))
  (if (Actor|ActorHasTag OtherActor "Wall")
    (Variables|Default|SetDirectionVector (Math|Vector|MakeVector (.x (Variables|Default|GetDirectionVector)) (* (.y (Variables|Default|GetDirectionVector)) -1.0) 0.0))
    (Transformation|SetActorRotation (Math|Rotator|FindLookatRotation (Math|Vector|MakeVector (.x _returnvalue) (.y _returnvalue) 0.0) (Math|Vector|MakeVector (.x (+ (Math|Vector|MakeVector (.x _returnvalue) (.y _returnvalue) (.z _returnvalue)) (Variables|Default|GetDirectionVector))) (.y (+ (Math|Vector|MakeVector (.x _returnvalue) (.y _returnvalue) (.z _returnvalue)) (Variables|Default|GetDirectionVector))) 0.0)))))

(event OnComponentBeginOverlap(XCollision)
  (params (OverlappedComponent :type Primitive%20Component%20Object%20Reference) (OtherActor :type Actor%20Object%20Reference) (OtherComp :type Primitive%20Component%20Object%20Reference) (OtherBodyIndex :type Integer) (bFromSweep :type Boolean) (SweepResult :type Hit%20Result%20Structure%20%28by%20ref%29))
  (bind _returnvalue (Transformation|GetActorLocation))
  (if (Actor|ActorHasTag OtherActor "Wall")
    (Variables|Default|SetDirectionVector (Math|Vector|MakeVector (* (.x (Variables|Default|GetDirectionVector)) -1.0) (.y (Variables|Default|GetDirectionVector)) 0.0))
    (Transformation|SetActorRotation (Math|Rotator|FindLookatRotation (Math|Vector|MakeVector (.x _returnvalue) (.y _returnvalue) 0.0) (Math|Vector|MakeVector (.x (+ (Math|Vector|MakeVector (.x _returnvalue) (.y _returnvalue) (.z _returnvalue)) (Variables|Default|GetDirectionVector))) (.y (+ (Math|Vector|MakeVector (.x _returnvalue) (.y _returnvalue) (.z _returnvalue)) (Variables|Default|GetDirectionVector))) 0.0)))))

(event OnComponentBeginOverlap(DamageCollision)
  (params (OverlappedComponent :type Primitive%20Component%20Object%20Reference) (OtherActor :type Actor%20Object%20Reference) (OtherComp :type Primitive%20Component%20Object%20Reference) (OtherBodyIndex :type Integer) (bFromSweep :type Boolean) (SweepResult :type Hit%20Result%20Structure%20%28by%20ref%29))
  (if (Utilities|DoesObjectImplementInterface OtherActor "/Game/Core/Character/BPI_PlayerInteraction.BPI_PlayerInteraction_C")
    (Class|BPIPlayerInteraction|Kill(Message) OtherActor)))

(event EventTick
  (params (DeltaSeconds :type Float%20%28single-precision%29))
  (bind _speed (Variables|Default|GetSpeed))
  (bind _directionvector (Variables|Default|GetDirectionVector))
  (bind _returnvalue (* DeltaSeconds _speed))
  (bind _returnvalue_2 (* _directionvector _returnvalue))
  (Transformation|AddActorWorldOffset (Math|Vector|MakeVector (.x _returnvalue_2) (.y _returnvalue_2) 0.0)))

(event EventBeginPlay
  (bind _returnvalue (Transformation|GetActorLocation))
  (Variables|Default|SetDirectionVector (Math|Vector|Normalize (Math|Vector|MakeVector (Math|Random|RandomFloatinRange -1.0 1.0) (Math|Random|RandomFloatinRange 0.0 1.0) 0.0)))
  (Transformation|SetActorRotation (Math|Rotator|FindLookatRotation (Math|Vector|MakeVector (.x _returnvalue) (.y _returnvalue) 0.0) (Math|Vector|MakeVector (.x (+ (Math|Vector|MakeVector (.x _returnvalue) (.y _returnvalue) (.z _returnvalue)) (Variables|Default|GetDirectionVector))) (.y (+ (Math|Vector|MakeVector (.x _returnvalue) (.y _returnvalue) (.z _returnvalue)) (Variables|Default|GetDirectionVector))) 0.0))))

(event EventInitRoundValues
  (params (RoundStats :type S%20Round%20Stat%20Structure))
  (Variables|Default|SetSpeed (.razorspeed RoundStats)))

(fn ConstructionScript
  (|CallParentFunction))