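; BP_Microwave is an enemy whose speed comes from round stats and which explodes after a timed fuse.
; ExplodingEffects plays sound and Niagara, opens a brief damage window, enables mesh physics, pulses a radial force and blackens the tint.
; While a player overlaps DamageCollision, a looping timer kills them if that window is open.
; After the window closes, the microwave deals itself damage through OnHurt; the floating timeline is never triggered.
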(event OnComponentBeginOverlap(DamageCollision)
  (params (OverlappedComponent :type Primitive%20Component%20Object%20Reference) (OtherActor :type Actor%20Object%20Reference) (OtherComp :type Primitive%20Component%20Object%20Reference) (OtherBodyIndex :type Integer) (bFromSweep :type Boolean) (SweepResult :type Hit%20Result%20Structure%20%28by%20ref%29))
  (if (Utilities|DoesObjectImplementInterface OtherActor "/Game/Core/Character/BPI_PlayerInteraction.BPI_PlayerInteraction_C")
    (bind _returnvalue (Utilities|Time|SetTimerbyEvent (delegate Custom|CheckIfCanHurt) 0.01 true true))
    (Variables|Default|SetPlayerReference OtherActor)
    (Variables|Default|SetCheckIfCanHurtTimer _returnvalue)))

(event OnComponentEndOverlap(DamageCollision)
  (params (OverlappedComponent :type Primitive%20Component%20Object%20Reference) (OtherActor :type Actor%20Object%20Reference) (OtherComp :type Primitive%20Component%20Object%20Reference) (OtherBodyIndex :type Integer))
  (if (Utilities|DoesObjectImplementInterface OtherActor "/Game/Core/Character/BPI_PlayerInteraction.BPI_PlayerInteraction_C")
    (Utilities|Time|ClearandInvalidateTimerbyHandle (Variables|Default|GetCheckIfCanHurtTimer))))

(event Custom|DeactivateExplosion
  (Components|Activation|Deactivate (Variables|Default|GetRadialForce)))

(event Custom|FuckingExplode
  (Utilities|ExplodingEffects)
  (Variables|Default|SetShouldFloat false)
  (Utilities|FlowControl|Delay 0.3)
  (Variables|Default|SetCanHurt false)
  (Utilities|FlowControl|Delay 0.5)
  (CallFunction|OnHurt 3e+02))

(event Custom|CheckIfCanHurt
  (if (and (Variables|Default|GetCanHurt) (Utilities|DoesObjectImplementInterface (Variables|Default|GetPlayerReference) "/Game/Core/Character/BPI_PlayerInteraction.BPI_PlayerInteraction_C"))
    (bind _asbpi_player_interaction (Utilities|Casting|CastToBPI_PlayerInteraction (Variables|Default|GetPlayerReference)))
    (Default|Kill _asbpi_player_interaction)))

(event EventExplode
  (Utilities|Time|SetTimerbyEvent (delegate Custom|FuckingExplode) (Variables|Default|GetExplodingTime)))

(event EventInitRoundValues
  (params (RoundStats :type S%20Round%20Stat%20Structure))
  (Utilities|FlowControl|Sequence
    (:then_0
      (Variables|/Script/Engine.CharacterMovementComponent|SetMaxWalkSpeed (Variables|Character|GetCharacterMovement) (.microwavespeed RoundStats)))))

(fn ConstructionScript
  (|CallParentFunction))