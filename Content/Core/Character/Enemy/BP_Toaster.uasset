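; BP_Toaster is a toaster enemy that fires projectiles at a repeating interval.
; A looping timer started on BeginPlay spawns BP_EnemyProjectile at the ProjectileArrow transform and sets its speed, with a leftover "fix shooting" debug print.
; LooktoPlayer rotates the actor toward the player pawn using only X/Y positions.
; InitRoundValues takes fire rate and projectile speed from round stats, without restarting the timer.
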(event Custom|ShootIIteration
  (bind _returnvalue (Game|SpawnActorfromClass "/Game/Core/Projectile/BP_EnemyProjectile.BP_EnemyProjectile_C" (Transformation|GetWorldTransform (Variables|Default|GetProjectileArrow)) "AlwaysSpawn" "MultiplyWithRoot" 0 self))
  (Default|SetProjectileSpeed _returnvalue (Variables|Default|GetProjectileSpeed))
  (Development|PrintString "TODO: fix shooting"))

(event EventLooktoPlayer
  (bind _returnvalue (Transformation|GetActorLocation))
  (bind _returnvalue_2 (Game|Player|GetPlayerPawn 0))
  (bind _returnvalue_3 (Transformation|GetActorLocation _returnvalue_2))
  (Transformation|SetActorRotation (Math|Rotator|FindLookatRotation (Math|Vector|MakeVector (.x _returnvalue) (.y _returnvalue) 0.0) (Math|Vector|MakeVector (.x _returnvalue_3) (.y _returnvalue_3) 0.0))))

(event EventBeginPlay
  (Utilities|Time|SetTimerbyEvent (delegate Custom|ShootIIteration) (Variables|Default|GetShootingRate) true))

(event EventInitRoundValues
  (params (RoundStats :type S%20Round%20Stat%20Structure))
  (Utilities|FlowControl|Sequence
    (:then_0
      (Variables|Default|SetShootingRate (.toastershootingrate RoundStats)))
    (:then_1
      (Variables|Default|SetProjectileSpeed (.toasterprojectilespeed RoundStats)))))

(fn ConstructionScript
  (|CallParentFunction))