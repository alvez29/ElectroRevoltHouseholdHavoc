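; Player controller that turns the player character to face the mouse cursor or gamepad stick direction.
; On BeginPlay it adds the Enhanced Input mapping context and caches the character through BPI_PlayerInteraction.
; Look inputs switch between Mouse and Controller modes, which Tick uses to pick the LookAt target.
; Mouse mode targets a cursor trace hit; Controller mode offsets from the pawn by the look stick, falling back to move input.
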(event Input|EnhancedActionEvents|EnhancedInputActionIPA_Look_Mouse
  (params (ActionValue :type Vector%202D%20Structure) (ElapsedSeconds :type Float%20%28double-precision%29) (TriggeredSeconds :type Float%20%28double-precision%29) (InputAction :type Input%20Action%20Object%20Reference :default "/Game/Input/IPA_Look_Mouse.IPA_Look_Mouse"))
  (:Started
    (Variables|Default|SetInputMode "NewEnumerator1")))

(event Input|EnhancedActionEvents|EnhancedInputActionIPA_Look_Joystick
  (params (ActionValue :type Vector%202D%20Structure) (ElapsedSeconds :type Float%20%28double-precision%29) (TriggeredSeconds :type Float%20%28double-precision%29) (InputAction :type Input%20Action%20Object%20Reference :default "/Game/Input/IPA_Look_Joystick.IPA_Look_Joystick"))
  (:Triggered
    (Variables|Default|SetLookJoystickVector (Math|Vector2D|MakeVector2D (.y ActionValue) (.x ActionValue))))
  (:Started
    (Variables|Default|SetInputMode "NewEnumerator0")
    (Variables|Default|SetIsMovingLookJoystick true))
  (:Canceled
    (Variables|Default|SetIsMovingLookJoystick false :!label _label))
  (:Completed
    (goto _label)))

(event Input|EnhancedActionEvents|EnhancedInputActionIPA_Move
  (params (ActionValue :type Vector%202D%20Structure) (ElapsedSeconds :type Float%20%28double-precision%29) (TriggeredSeconds :type Float%20%28double-precision%29) (InputAction :type Input%20Action%20Object%20Reference :default "/Game/Input/IPA_Move.IPA_Move"))
  (Variables|Default|SetMoveJoysticVector ActionValue))

(event EventTick
  (params (DeltaSeconds :type Float%20%28single-precision%29))
  (switch Utilities|FlowControl|Switch|SwitchonE_InputType (Variables|Default|GetInputMode)
    (:NewEnumerator0
      (if (Variables|Default|GetIsMovingLookJoystick)
        (Utilities|ProcessControllerTick :!label _label)
        (else
          (goto _label Moving))))
    (:NewEnumerator1
      (Variables|Default|SetCursorLocation (.Location (CallFunction|GetLocationUnderCursor)))
      (Utilities|ProcessMouseTick))))

(event EventBeginPlay
  (bind _returnvalue (PlayerController|LocalPlayerSubsystems|GetEnhancedInputLocalPlayerSubsystem))
  (Utilities|IsValid _returnvalue
    (:Is%20Valid
      (Input|AddMappingContext _returnvalue "/Game/Input/IMC_Player.IMC_Player" 0 "(bIgnoreAllPressedKeysUntilRelease=True,bForceImmediately=False,bNotifyUserSettings=False)")
      (bind _asbpi_player_interaction (Utilities|Casting|CastToBPI_PlayerInteraction (Game|GetPlayerCharacter 0)))
      (Variables|Default|SetPlayerReference _asbpi_player_interaction)
      (Input|SetInputModeGameandUI self 0 "DoNotLock" false false))))

(fn ConstructionScript)

(fn GetLocationUnderCursor
  (bind _hitresult (Game|Player|GetHitResultUnderCursorbyChannel "TraceTypeQuery3" true))
  (bind (_bblockinghit _binitialoverlap _time _distance _location) (Collision|BreakHitResult _hitresult))
  (return _bblockinghit _location))